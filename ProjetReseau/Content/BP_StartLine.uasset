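; BP_StartLine is a race start/finish line whose box overlap counts laps for BP_VehicleAdvPawnBase vehicles, on the server only.
; It skips vehicles flagged IsFirstTime; that branch re-sets the flag to true rather than clearing it.
; Otherwise it opens Lvl_ThirdPerson if Laps has reached MaxLaps, or increments Laps.
; A single DoOnce with a delayed reset debounces increments across all vehicles.
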(event `self.Box.OnComponentBeginOverlap`
  (params (OverlappedComponent :type "PrimitiveComponent Object Reference") (OtherActor :type "Actor Object Reference") (OtherComp :type "PrimitiveComponent Object Reference") (OtherBodyIndex :type Integer) (bFromSweep :type Boolean) (SweepResult :type "HitResult Structure (by ref)"))
  (`/Engine/EditorBlueprintResources/ActorMacros.Switch Has Authority`
    (:`Authority`
      (bind _asbp_vehicle_adv_pawn_base (cast `/Game/VehicleTemplate/Blueprints/BP_VehicleAdvPawnBase` OtherActor))
      (if (`/Game/VehicleTemplate/Blueprints/BP_VehicleAdvPawnBase.Is First Time` _asbp_vehicle_adv_pawn_base)
        (set `/Game/VehicleTemplate/Blueprints/BP_VehicleAdvPawnBase.Is First Time` true _asbp_vehicle_adv_pawn_base)
        (else
          (bind _laps (`/Game/VehicleTemplate/Blueprints/BP_VehicleAdvPawnBase.Laps` _asbp_vehicle_adv_pawn_base))
          (if (>= _laps (`/Game/VehicleTemplate/Blueprints/BP_VehicleAdvPawnBase.Max Laps` _asbp_vehicle_adv_pawn_base))
            (`GameplayStatics.OpenLevelBySoftObjectPtr` "/Game/ThirdPerson/Lvl_ThirdPerson.Lvl_ThirdPerson")
            (else
              (`/Engine/EditorBlueprintResources/StandardMacros.DoOnce` false :!label _label
                (:`Completed`
                  (set `/Game/VehicleTemplate/Blueprints/BP_VehicleAdvPawnBase.Laps` (+ _laps 1) _asbp_vehicle_adv_pawn_base)
                  (`KismetSystemLibrary.Delay` 0.7)
                  (goto _label :!via `Reset`))))))))))

(fn `UserConstructionScript`)